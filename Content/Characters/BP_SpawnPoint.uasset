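; BP_SpawnPoint populates an area with Rat_BP characters, spawning a set amount at BeginPlay.
; Each spawn line-traces from high above a random point in the Bounds component toward an absolute, not start-relative, end point, placing the rat above the hit.
; Rats get a default controller and spawn point reference, then join ActivePawns.
; A looping timer spawns one more whenever that array is below SpawnAmount; removal happens outside this Blueprint.
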(event `self.ReceiveBeginPlay`
  (for _ (range 1 (+ (`self.SpawnAmount`) 1))
    (`self.SpawnCharacter`))
  (`KismetSystemLibrary.K2_SetTimer` null "RespawnCharacter" (`self.TimeTilRespawn`) true))

(fn `RespawnCharacter`
  (if (< (`KismetArrayLibrary.Array_Length` (`self.ActivePawns`)) (`self.SpawnAmount`))
    (`self.SpawnCharacter`)))

(fn `SpawnCharacter`
  (bind (_origin _boxextent) (`KismetSystemLibrary.GetComponentBounds` (`self.Bounds`)))
  (bind _outhit (`KismetSystemLibrary.LineTraceSingleForObjects` :`Start` (`KismetMathLibrary.MakeVector` (.x (`KismetMathLibrary.RandomPointInBoundingBox` _origin _boxextent)) (.y (`KismetMathLibrary.RandomPointInBoundingBox` _origin _boxextent)) (+ (.z (`KismetMathLibrary.RandomPointInBoundingBox` _origin _boxextent)) 10000.0)) :`End` (* (* (`self.GetActorUpVector`) -1) 15000.0) :`ObjectTypes` (`|MakeArray` "ObjectTypeQuery1" :!type "EObjectTypeQuery Enum") :`DrawDebugType` "ForDuration"))
  (bind _returnvalue (`|SpawnActorFromClass` "/Game/Characters/Rat/Rat_BP.Rat_BP_C" (`KismetMathLibrary.MakeTransform` (`KismetMathLibrary.MakeVector` (.x (`.ImpactPoint` (`GameplayStatics.BreakHitResult` _outhit))) (.y (`.ImpactPoint` (`GameplayStatics.BreakHitResult` _outhit))) (+ (.z (`.ImpactPoint` (`GameplayStatics.BreakHitResult` _outhit))) 100.0)) (`KismetMathLibrary.MakeRotator` 0.0 0.0 (`KismetMathLibrary.RandomFloat`))) "AdjustIfPossibleButAlwaysSpawn" "OverrideRootScale" null null))
  (`Pawn.SpawnDefaultController` _returnvalue)
  (set `/Game/Characters/Rat/Rat_BP.Spawn Point` self _returnvalue)
  (`KismetArrayLibrary.Array_Add` (`self.ActivePawns`) _returnvalue))

(fn `UserConstructionScript`)